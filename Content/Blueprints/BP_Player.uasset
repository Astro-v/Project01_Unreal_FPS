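; BP_Player is the player Blueprint, handling movement, look rotation and projectile firing.
; Axis inputs move it along directions yawed by the Arrow component, while look inputs rotate Sphere1 in world yaw and around Arrow's right axis for pitch, scaled by per-axis speeds.
; Pressing FireProjectile spawns BP_Projectile at Arrow1's transform and passes that arrow's forward unit vector to SetVelocityInLocalSpace on its ProjectileMovement.
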(event Input|ActionEvents|InputActionFireProjectile
  (params (Key :type Key%20Structure :default "None"))
  (bind _arrow1 (Variables|Default|GetArrow1))
  ;[1 1 1] Projectile
  (:Pressed
    (bind _returnvalue (Game|SpawnActorfromClass "/Game/Blueprints/BP_Projectile.BP_Projectile_C" (Transformation|GetWorldTransform _arrow1) "Undefined" 0 0))
    (Game|Components|ProjectileMovement|SetVelocityinLocalSpace (Variables|/Game/Blueprints/BP_Projectile.BP_Projectile_C|GetProjectileMovement _returnvalue) (Math|Vector|RotateVector (Math|Vector|MakeVector 1.0 0.0 0.0) (.rotation (Transformation|GetWorldTransform _arrow1))))))

(event Input|AxisEvents|InputAxisRotateCameraX
  (params (AxisValue :type Float%20%28single-precision%29))
  ;[1 1 1] Rotation system
  (Transformation|AddWorldRotation (Variables|Default|GetSphere1) (Math|Rotator|MakeRotator 0.0 0.0 (* AxisValue (Variables|Default|GetRotationSpeedX))) false false))

(event Input|AxisEvents|InputAxisMoveForward
  (params (AxisValue :type Float%20%28single-precision%29))
  ;[1 1 1] Movement system
  (Pawn|Input|AddMovementInput (Math|Vector|RotateVector (Math|Vector|MakeVector 1.0 0.0 0.0) (Math|Rotator|MakeRotator 0.0 0.0 (.yaw (.rotation (Transformation|GetWorldTransform (Variables|Default|GetArrow)))))) AxisValue false))

(event Input|AxisEvents|InputAxisMoveSide
  (params (AxisValue :type Float%20%28single-precision%29))
  ;[1 1 1] Movement system
  (Pawn|Input|AddMovementInput (Math|Vector|RotateVector (Math|Vector|MakeVector 0.0 1.0 0.0) (Math|Rotator|MakeRotator 0.0 0.0 (.yaw (.rotation (Transformation|GetWorldTransform (Variables|Default|GetArrow)))))) AxisValue false))

(event Input|AxisEvents|InputAxisRotateCameraY
  (params (AxisValue :type Float%20%28single-precision%29))
  ;[1 1 1] Rotation system
  (Transformation|AddWorldRotation (Variables|Default|GetSphere1) (Math|Vector|RotatorfromAxisandAngle (Math|Vector|RotateVector (Math|Vector|MakeVector 0.0 1.0 0.0) (.rotation (Transformation|GetWorldTransform (Variables|Default|GetArrow)))) (* AxisValue (Variables|Default|GetRotationSpeedY))) false false))

(fn ConstructionScript)